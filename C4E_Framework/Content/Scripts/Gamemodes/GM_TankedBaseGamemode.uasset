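; Base gamemode for Tanked that runs a set of objective rules and ends the game when they are met.
; Child gamemodes override RegisterGameRules to fill ActiveRules, which BeginPlay initializes, binds for completion and passes to an objective UI widget.
; A successful major rule ends the game at once, while other successes end it only when every rule is completed.
; Ending quits the game after a brief delay.
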(event `self.ReceiveBeginPlay`
  (`self.RegisterGameRules`)
  (if (`KismetArrayLibrary.Array_IsNotEmpty` (`self.ActiveRules`))
    (for (_array_element _array_index) (`self.ActiveRules`)
      (`/Game/Scripts/Gamemodes/Rules/BPC_BaseGameRule.InitRule` _array_element _array_index)
      (add `/Game/Scripts/Gamemodes/Rules/BPC_BaseGameRule.ERuleComplete` _array_element (`|CreateDelegate` :!event `OnRuleCompleted`)))
    (bind _returnvalue (`|CreateWidget` "/Game/Scripts/UI/WBP_ObjectiveUI.WBP_ObjectiveUI_C"))
    (`/Game/Scripts/UI/WBP_ObjectiveUI.InitRules` _returnvalue (`self.ActiveRules`))
    (`UserWidget.AddToViewport` _returnvalue 0)))

(event `RegisterGameRules`)

(event `OnRuleCompleted`
  (params (RuleID :type Integer) (bSuccessful :type Boolean))
  (bind _brulescompleted (`self.CheckRules` RuleID bSuccessful))
  (if _brulescompleted
    (`self.EndGame`)))

(event `EndGame`
  (`KismetSystemLibrary.Delay` 0.2)
  (`KismetSystemLibrary.QuitGame` null "Quit"))

(fn `CheckRules`
  (params (RuleID :type Integer) (bSuccessful :type Boolean))
  (returns (bRulesCompleted :type Boolean))
  (if bSuccessful
    (if (`/Game/Scripts/Gamemodes/Rules/BPC_BaseGameRule.MajorRule` (`|GetArrayItem` (`self.ActiveRules`) RuleID))
      (return true)
      (else
        (for _array_element (`self.ActiveRules`)
          (if (not (`/Game/Scripts/Gamemodes/Rules/BPC_BaseGameRule.Completed` _array_element))
            (return false)))
        (return true)))))

(fn `UserConstructionScript`)