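; Game rule component for gamemodes that completes the rule when a countdown of TimerLength runs out.
; InitRule starts the main timer plus a looping one-second timer, which broadcasts the remaining time through event dispatchers alongside start and completion notifications.
; When time expires, it clears the tick timer, flags Completed and calls CompleteRule.
; Add and deduct events adjust a running countdown by setting the timer again with the adjusted remaining time.
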(event `self.InitRule`
  (params (ID :type Integer))
  (`parent.InitRule` ID)
  (`|ExecutionSequence`
    (:`then_0`
      (bind _returnvalue (`KismetSystemLibrary.K2_SetTimerDelegate` (`|CreateDelegate` :!event `TimerEnded`) (`self.TimerLength`))) ; Create overarching timer of provided length
      (set `self.Timer` _returnvalue))
    (:`then_1`
      (bind _returnvalue_2 (`KismetSystemLibrary.K2_SetTimerDelegate` (`|CreateDelegate` :!event `TimerCheck`) 1.0 true)) ; Create a timer to check elapased time every second
      (set `self.TimerCheckTimer` _returnvalue_2))
    (:`then_2`
      (`self.ETimerStarted`) ; Fire event to note that the timer has started
    )))

(event `TimerCheck`
  (bind _returnvalue (`KismetSystemLibrary.K2_GetTimerRemainingTimeHandle` (`self.Timer`)))
  (if (> _returnvalue 0.0)
    (`self.ETimerTicked` _returnvalue)))

(event `TimerEnded`
  (`KismetSystemLibrary.K2_ClearAndInvalidateTimerHandle` (`self.TimerCheckTimer`)) ; Clear timer which fires every second
  (`self.ETimerCompleted`)
  (set `self.Completed` true)
  (`self.CompleteRule`))

(event `Add to Timer`
  (params (`Seconds to Add` :type "Float (double-precision)"))
  (bind _returnvalue (`KismetSystemLibrary.K2_GetTimerRemainingTimeHandle` (`self.Timer`)))
  (if (> _returnvalue 0.0)
    (bind _returnvalue_2 (`KismetSystemLibrary.K2_SetTimerDelegate` (`|CreateDelegate` :!event `TimerEnded`) (+ _returnvalue `Seconds to Add`)))
    (set `self.Timer` _returnvalue_2)))

(event `Deduct from Timer`
  (params (`Seconds to Remove` :type "Float (double-precision)"))
  (bind _returnvalue (`KismetSystemLibrary.K2_GetTimerRemainingTimeHandle` (`self.Timer`)))
  (if (> _returnvalue 0.0)
    (bind _returnvalue_2 (`KismetSystemLibrary.K2_SetTimerDelegate` (`|CreateDelegate` :!event `TimerEnded`) (- _returnvalue `Seconds to Remove`)))
    (set `self.Timer` _returnvalue_2)))