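; BP_TankShot is a short-lived tank shot actor that damages what it hits.
; On BeginPlay a timer starts that spawns a fail particle effect and destroys the shot if it expires first.
; The first overlap on its Sphere, gated by a DoOnce, applies damage to the other actor, spawns a scaled-down rocket explosion and destroys the shot.
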(event `self.ReceiveBeginPlay`
  (`KismetSystemLibrary.K2_SetTimerDelegate` (delegate `Killshot`) 0.75))

(event `Killshot`
  (bind (_returnvalue_location _returnvalue_rotation) (`KismetMathLibrary.BreakTransform` (`self.GetTransform`)))
  (`GameplayStatics.SpawnEmitterAtLocation` "/Game/Assets/Effects/PS_TankShotFail.PS_TankShotFail" _returnvalue_location _returnvalue_rotation)
  (`self.K2_DestroyActor`))

(event `self.Sphere.OnComponentBeginOverlap`
  (params (OverlappedComponent :type "PrimitiveComponent Object Reference") (OtherActor :type "Actor Object Reference") (OtherComp :type "PrimitiveComponent Object Reference") (OtherBodyIndex :type Integer) (bFromSweep :type Boolean) (SweepResult :type "HitResult Structure (by ref)"))
  (`/Engine/EditorBlueprintResources/StandardMacros.DoOnce` false
    (:`Completed`
      (`GameplayStatics.ApplyDamage` OtherActor 1.0)
      (`GameplayStatics.SpawnEmitterAtLocation` "/Game/Assets/Effects/PS_RocketExplosion.PS_RocketExplosion" (`self.K2_GetActorLocation`) (struct) (0.5 0.5 0.5))
      (`self.K2_DestroyActor`))))

(fn `UserConstructionScript`)