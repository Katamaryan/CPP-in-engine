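; BP_EndPoint is an objective end point that signals when a BP_Tank reaches it.
; With AutoActivate set, it is active from BeginPlay; otherwise its mesh is hidden and sphere collision disabled until Interact is triggered.
; Activation shows the mesh, enables query-only sphere collision and fires EEndActivated.
; A tank beginning overlap with the sphere fires EEndReached.
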(event `self.ReceiveBeginPlay`
  (bind _bautoactivate (`self.bAutoActivate`))
  (`SceneComponent.SetVisibility` (`self.StaticMesh`) _bautoactivate false)
  (`PrimitiveComponent.SetCollisionEnabled` (`self.Sphere`) (select `bool` _bautoactivate :`false` "NoCollision" :`true` "QueryOnly" :!type "ECollisionEnabled Enum"))
  (if (`self.bAutoActivate`)
    (`self.EEndActivated`)))

(event `/Game/Scripts/Interfaces/BPI_Interact.Interact`
  (params (InteractorPawn :type "Pawn Object Reference"))
  (if (not (`self.bAutoActivate`))
    (`SceneComponent.SetVisibility` (`self.StaticMesh`) true false)
    (`PrimitiveComponent.SetCollisionEnabled` (`self.Sphere`) "QueryOnly")
    (`self.EEndActivated`)))

(event `self.Sphere.OnComponentBeginOverlap`
  (params (OverlappedComponent :type "PrimitiveComponent Object Reference") (OtherActor :type "Actor Object Reference") (OtherComp :type "PrimitiveComponent Object Reference") (OtherBodyIndex :type Integer) (bFromSweep :type Boolean) (SweepResult :type "HitResult Structure (by ref)"))
  (cast `/Game/Scripts/Pawns/BP_Tank` OtherActor)
  (`self.EEndReached`))

(fn `UserConstructionScript`)