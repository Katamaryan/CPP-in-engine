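; Rocket turret enemy that extends a parent enemy class and fires BP_Rocket projectiles at the player tank referenced by TankREF.
; TurretFire alternates between two arrow muzzles via the Point flag, taking pitch from a look-at just below the tank and yaw from the arrow.
; Each shot triggers MachineGunShake, where timelines jolt the turret and one of two launcher meshes, then calls the parent fire logic.
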(event `self.ReceiveBeginPlay`
  (`parent.ReceiveBeginPlay`))

(event `self.ReceiveTick`
  (params (DeltaSeconds :type "Float (single-precision)"))
  (`parent.ReceiveTick` DeltaSeconds))

(event `MachineGunShake`
  (bind _turretspin (`self.TurretSpin`))
  (bind (_relativerotation_roll _relativerotation_pitch _relativerotation_yaw) (`KismetMathLibrary.BreakRotator` (`SceneComponent.RelativeRotation` _turretspin)))
  (`|ExecutionSequence`
    (:`then_0`
      (bind (_direction _turret_movement) (`Timeline|GunShake` :!via `PlayFromStart`)
        (:`Update`
          (`SceneComponent.K2_SetRelativeLocationAndRotation` _turretspin (`KismetMathLibrary.MakeVector` 0.0 0.0 (+ _turret_movement 7.0)) (`KismetMathLibrary.MakeRotator` 0.0 (- 0.0 _turret_movement) _relativerotation_yaw) false false))))
    (:`then_1`
      (if (`self.Point`)
        (bind (_direction_2 _newtrack_0) (`Timeline|RocketShake` :!via `PlayFromStart`)
          (:`Update`
            (`SceneComponent.K2_SetRelativeLocation` (`self.StaticMesh_0`) (`KismetMathLibrary.MakeVector` 0.0 _newtrack_0) false false)))
        (else
          (bind (_direction_3 _newtrack_0_2) (`Timeline|Timeline_0` :!via `PlayFromStart`)
            (:`Update`
              (`SceneComponent.K2_SetRelativeLocation` (`self.StaticMesh1`) (`KismetMathLibrary.MakeVector` 0.0 _newtrack_0_2) false false))))))))

(fn `Turret Fire`
  (bind _arrow (`self.Arrow`))
  (bind _arrow1 (`self.Arrow1`))
  (bind (_returnvalue_x _returnvalue_y _returnvalue_z) (`KismetMathLibrary.BreakVector` (`self.K2_GetActorLocation` (`self.TankREF`))))
  (bind _returnvalue (`SceneComponent.K2_GetComponentLocation` _arrow))
  (bind (_returnvalue_roll _returnvalue_pitch _returnvalue_yaw) (`KismetMathLibrary.BreakRotator` (`SceneComponent.K2_GetComponentRotation` _arrow1)))
  (bind (_returnvalue_roll_2 _returnvalue_pitch_2 _returnvalue_yaw_2) (`KismetMathLibrary.BreakRotator` (`SceneComponent.K2_GetComponentRotation` _arrow)))
  (bind _returnvalue_2 (`SceneComponent.K2_GetComponentLocation` _arrow1))
  (bind _returnvalue_3 (`KismetMathLibrary.MakeVector` _returnvalue_x _returnvalue_y (- _returnvalue_z 20.0)))
  (bind (_returnvalue_roll_3 _returnvalue_pitch_3) (`KismetMathLibrary.BreakRotator` (`KismetMathLibrary.FindLookAtRotation` _returnvalue_2 _returnvalue_3)))
  (bind (_returnvalue_roll_4 _returnvalue_pitch_4) (`KismetMathLibrary.BreakRotator` (`KismetMathLibrary.FindLookAtRotation` _returnvalue _returnvalue_3)))
  (if (`self.Point`)
    (set `self.Point` false)
    (`|SpawnActorFromClass` "/Game/Scripts/Gameplay/Weapons/BP_Rocket.BP_Rocket_C" (`KismetMathLibrary.MakeTransform` _returnvalue (`KismetMathLibrary.MakeRotator` _returnvalue_roll_2 _returnvalue_pitch_4 _returnvalue_yaw_2)) "Undefined" "OverrideRootScale" null null)
    (else
      (set `self.Point` true)
      (`|SpawnActorFromClass` "/Game/Scripts/Gameplay/Weapons/BP_Rocket.BP_Rocket_C" (`KismetMathLibrary.MakeTransform` _returnvalue_2 (`KismetMathLibrary.MakeRotator` _returnvalue_roll _returnvalue_pitch_3 _returnvalue_yaw)) "Undefined" "OverrideRootScale" null null)))
  (`self.MachineGunShake`)
  (`parent.Turret Fire`))

(fn `UserConstructionScript`
  (`parent.UserConstructionScript`))