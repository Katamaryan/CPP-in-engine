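; Machine gun turret enemy that overrides its parent's fire logic with an instant hitscan shot.
; TurretFire line-traces forward from the Arrow, damages any hit actor and spawns a small explosion at the impact.
; A beam particle is drawn to the impact point, or to the trace's end on a miss.
; Each shot replays the GunShake timeline to jolt and pitch TurretSpin, then calls the parent's TurretFire.
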(event `self.ReceiveBeginPlay`
  (`parent.ReceiveBeginPlay`))

(event `self.ReceiveTick`
  (params (DeltaSeconds :type "Float (single-precision)"))
  (`parent.ReceiveTick` DeltaSeconds))

(event `MachineGunShake`
  (bind _turretspin (`self.TurretSpin`))
  (bind (_relativerotation_roll _relativerotation_pitch _relativerotation_yaw) (`KismetMathLibrary.BreakRotator` (`SceneComponent.RelativeRotation` _turretspin)))
  (bind (_direction _turret_movement) (`Timeline|GunShake` :!via `PlayFromStart`)
    (:`Update`
      (`SceneComponent.K2_SetRelativeLocationAndRotation` _turretspin (`KismetMathLibrary.MakeVector` 0.0 0.0 (+ _turret_movement 7.0)) (`KismetMathLibrary.MakeRotator` 0.0 (- 0.0 _turret_movement) _relativerotation_yaw) false false))))

(fn `Turret Fire`
  (bind _arrow (`self.Arrow`))
  (bind _returnvalue (`SceneComponent.K2_GetComponentLocation` _arrow))
  (bind _returnvalue_2 (+ _returnvalue (* (`SceneComponent.GetForwardVector` _arrow) 500.0)))
  (bind (_outhit _returnvalue_3) (`KismetSystemLibrary.LineTraceSingle` _returnvalue _returnvalue_2 "TraceTypeQuery1"))
  (if _returnvalue_3
    (bind (_bblockinghit _binitialoverlap _time _distance _location _impactpoint _normal _impactnormal _physmat _hitactor) (`GameplayStatics.BreakHitResult` _outhit))
    (`GameplayStatics.ApplyDamage` _hitactor 1.0)
    (bind _returnvalue_4 (`GameplayStatics.SpawnEmitterAtLocation` "/Game/Assets/Effects/PS_LineTraceBeam.PS_LineTraceBeam" (`SceneComponent.K2_GetComponentLocation` (`self.Arrow`))))
    (`ParticleSystemComponent.SetBeamTargetPoint` _returnvalue_4 0 _impactpoint 0)
    (`GameplayStatics.SpawnEmitterAtLocation` "/Game/Assets/Effects/PS_RocketExplosion.PS_RocketExplosion" _impactpoint (struct) (0.25 0.25 0.25))
    (else
      (bind _returnvalue_5 (`GameplayStatics.SpawnEmitterAtLocation` "/Game/Assets/Effects/PS_LineTraceBeam.PS_LineTraceBeam" (`SceneComponent.K2_GetComponentLocation` (`self.Arrow`))))
      (`ParticleSystemComponent.SetBeamTargetPoint` _returnvalue_5 0 _returnvalue_2 0)))
  (`self.MachineGunShake`)
  (`parent.Turret Fire`))

(fn `UserConstructionScript`
  (`parent.UserConstructionScript`))