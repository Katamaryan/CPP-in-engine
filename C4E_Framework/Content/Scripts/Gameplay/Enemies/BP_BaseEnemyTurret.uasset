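; Base enemy turret that tracks the player tank, fires when its range check hits, and explodes on death.
; Tick smoothly yaws TurretSpin toward the cached BP_CPPTank, while a randomly staggered looping timer drives a sphere trace that calls TurretFire, an empty stub here.
; HealthComponent's death event handles destruction, and the construction script initializes health and scales the DangerZone to Range.
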(event `self.ReceiveBeginPlay`
  (bind _healthcomponent (`self.HealthComponent`))
  (`/Game/Scripts/Components/BPC_HealthComponent.ResetHealth` _healthcomponent)
  (add `/Game/Scripts/Components/BPC_HealthComponent.EDeath` _healthcomponent (`|CreateDelegate` :!event `TurretDestroyed`))
  (bind _outactors (`GameplayStatics.GetAllActorsOfClass` "/Game/StudentWork/BP_CPPTank.BP_CPPTank_C"))
  (for _array_element _outactors
    (set `self.TankREF` _array_element))
  (`KismetSystemLibrary.Delay` (`KismetMathLibrary.RandomFloatInRange` 0.0 0.9))
  (`KismetSystemLibrary.K2_SetTimerDelegate` (`|CreateDelegate` :!event `Fire`) (`self.FireRate`) true))

(event `Fire`
  (bind _returnvalue (`self.K2_GetActorLocation`))
  (bind (_outhits _returnvalue_2) (`KismetSystemLibrary.SphereTraceMulti` _returnvalue (+ _returnvalue (0.0 0.0 1.0)) (`self.Range`) "TraceTypeQuery3"))
  (if _returnvalue_2
    (`self.Turret Fire`)))

(event `TurretDestroyed`
  (params (Instigator :type "Controller Object Reference") (Causer :type "Actor Object Reference"))
  (`GameplayStatics.SpawnEmitterAtLocation` "/Game/Assets/Effects/PS_EnemyDeathExplosion.PS_EnemyDeathExplosion" (`self.K2_GetActorLocation`))
  (`self.K2_DestroyActor`))

(event `self.ReceiveTick`
  (params (DeltaSeconds :type "Float (single-precision)"))
  (bind _turretspin (`self.TurretSpin`))
  (bind _tankref (`self.TankREF`))
  (bind (_returnvalue_roll _returnvalue_pitch _returnvalue_yaw) (`KismetMathLibrary.BreakRotator` (`KismetMathLibrary.RInterpTo` (`SceneComponent.K2_GetComponentRotation` _turretspin) (`KismetMathLibrary.FindLookAtRotation` (`SceneComponent.K2_GetComponentLocation` _turretspin) (`self.K2_GetActorLocation` _tankref)) (`GameplayStatics.GetWorldDeltaSeconds`) 2.0)))
  (`/Engine/EditorBlueprintResources/StandardMacros.IsValid` _tankref
    (:`Is Valid`
      (`SceneComponent.K2_SetWorldRotation` _turretspin (`KismetMathLibrary.MakeRotator` 0.0 0.0 _returnvalue_yaw) false false))))

(fn `Turret Fire`
  (return))

(fn `UserConstructionScript`
  (bind (_returnvalue_x _returnvalue_y) (`KismetMathLibrary.BreakVector` (`KismetMathLibrary.Conv_DoubleToVector` (`self.Range`))))
  (set `self.Health` (`self.MaxHP`))
  (`SceneComponent.SetWorldScale3D` (`self.DangerZone`) (`KismetMathLibrary.MakeVector` _returnvalue_x _returnvalue_y 50.0)))