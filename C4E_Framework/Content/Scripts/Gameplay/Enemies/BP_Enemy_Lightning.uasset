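; Lightning turret enemy that damages pawns around it with a radial electric blast, built on a parent Blueprint.
; Its Turret Fire override starts the GunShake timeline, then calls the parent logic.
; The timeline bobs and pitches TurretSpin while ramping two charge particle effects.
; Its FIRE event spawns the blast, sphere-traces pawns within Range, then applies fixed damage and an attached hit effect to each hit.
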(event `self.ReceiveBeginPlay`
  (`parent.ReceiveBeginPlay`))

(event `self.ReceiveTick`
  (params (DeltaSeconds :type "Float (single-precision)"))
  (`parent.ReceiveTick` DeltaSeconds))

(event `MachineGunShake`
  (bind _returnvalue (`self.K2_GetActorLocation`))
  (bind _turretspin (`self.TurretSpin`))
  (bind _lightingcharge (`self.LightingCharge`))
  (bind _lightingcharge1 (`self.LightingCharge1`))
  (bind (_relativerotation_roll _relativerotation_pitch _relativerotation_yaw) (`KismetMathLibrary.BreakRotator` (`SceneComponent.RelativeRotation` _turretspin)))
  (`|ExecutionSequence`
    (:`then_0`
      (bind (_direction _turret_movement _fx_buildup) (`Timeline|GunShake` :!via `PlayFromStart`)
        (:`Update`
          (`SceneComponent.K2_SetRelativeLocationAndRotation` _turretspin (`KismetMathLibrary.MakeVector` 0.0 0.0 (+ (* 5 _turret_movement) 7.0)) (`KismetMathLibrary.MakeRotator` 0.0 (- 0.0 _turret_movement) _relativerotation_yaw) false false)
          (`|ExecutionSequence`
            (:`then_0`
              (bind _returnvalue_2 (* _fx_buildup 40.0))
              (`FXSystemComponent.SetFloatParameter` _lightingcharge "LT1" _returnvalue_2)
              (bind _returnvalue_3 (* _fx_buildup 300.0))
              (`FXSystemComponent.SetFloatParameter` _lightingcharge "LT2" _returnvalue_3))
            (:`then_1`
              (`FXSystemComponent.SetFloatParameter` _lightingcharge1 "LT1" _returnvalue_2)
              (`FXSystemComponent.SetFloatParameter` _lightingcharge1 "LT2" _returnvalue_3))))
        (:`FIRE`
          (`GameplayStatics.SpawnEmitterAtLocation` "/Game/Assets/Effects/PS_LightingBlast.PS_LightingBlast" _returnvalue)
          (bind _outhits (`KismetSystemLibrary.SphereTraceMultiForObjects` _returnvalue (+ _returnvalue (0.0 0.0 1.0)) (`self.Range`) (`|MakeArray` "ObjectTypeQuery3" :!type "EObjectTypeQuery Enum")))
          (for _array_element _outhits
            (bind (_bblockinghit _binitialoverlap _time _distance _location _impactpoint _normal _impactnormal _physmat _hitactor _hitcomponent) (`GameplayStatics.BreakHitResult` _array_element))
            (`GameplayStatics.ApplyDamage` _hitactor 5.0)
            (`GameplayStatics.SpawnEmitterAttached` "/Game/Assets/Effects/PS_LightningHit.PS_LightningHit" _hitcomponent "None" (0.0 0.0 0.0) (struct) (1.0 1.0 1.0) "SnapToTarget")))))))

(fn `Turret Fire`
  (`self.MachineGunShake`)
  (`parent.Turret Fire`))

(fn `UserConstructionScript`
  (`parent.UserConstructionScript`))