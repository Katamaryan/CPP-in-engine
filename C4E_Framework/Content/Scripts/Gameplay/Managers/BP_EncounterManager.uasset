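; Encounter manager that starts and tracks target-destruction encounters when a BP_Tank overlaps mapped trigger volumes.
; Each trigger maps to an encounter ID and loses collision after tank entry; activation binds and activates the encounter actors' BPC_TargetComponents.
; Destroyed targets decrement a count until the encounter completes and is recorded.
; Start and end fire interactor messages, with dispatchers reporting start, count updates, end and completion of all encounters.
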(event `self.ReceiveBeginPlay`
  (bind _keys (`BlueprintMapLibrary.Map_Keys` (`self.EncounterTriggers`)))
  (for _array_element _keys
    (add `self.OnActorBeginOverlap` _array_element (`|CreateDelegate` :!event `OnEncounterTriggered`))))

(event `OnEncounterTriggered` :!signature `self.OnActorBeginOverlap`
  (params (OverlappedActor :type "Actor Object Reference") (OtherActor :type "Actor Object Reference"))
  (if (`.bSuccess` (cast `/Game/Scripts/Pawns/BP_Tank` OtherActor :!pure true))
    (bind _astrigger_base (cast `TriggerBase` OverlappedActor))
    (bind (_value _returnvalue) (`BlueprintMapLibrary.Map_Find` (`self.EncounterTriggers`) _astrigger_base))
    (if _returnvalue
      (`self.ActivateEncounter` _value))
    (`self.SetActorEnableCollision` _astrigger_base false)))

(event `OnTargetDestroyed`
  (bind _currenttargetcount (`self.CurrentTargetCount`))
  (bind _result (`/Engine/EditorBlueprintResources/StandardMacros.DecrementInt` _currenttargetcount)
    (:`  `
      (if (<= _result 0)
        (`self.EncounterCompleted`)
        (else
          (`self.ETargetCountUpdated` _currenttargetcount))))))

(event `EncounterCompleted`
  (set `self.CurrentTargetCount` 0)
  (`KismetArrayLibrary.Array_Add` (`self.CompletedEncounters`) (`.EncounterID_4_43AAB3D6462D385923557487844DF66A` (break `/Game/Scripts/Data/S_Encounter` (`self.TargetEncounter`))))
  (`KismetSystemLibrary.PrintString` "Encounter Completed")
  (`self.EEncounterEnded`)
  (for _array_element (`.EndInteractors_20_A8400C534BF7DE583690E6B2F375671C` (break `/Game/Scripts/Data/S_Encounter` (`self.TargetEncounter`)))
    (message `/Game/Scripts/Interfaces/BPI_Interact.Interact` _array_element null))
  (setmembers `/Game/Scripts/Data/S_Encounter` :`StructRef` (`self.TargetEncounter`) :`EncounterID` -1)
  (if (== (`KismetArrayLibrary.Array_Length` (`self.LevelEncounters`)) (`KismetArrayLibrary.Array_Length` (`self.CompletedEncounters`)))
    (`self.EEncountersCompleted`)))

(fn `ActivateEncounter`
  (params (EncounterID :type Integer))
  (bind ((`EncounterID_4_43AAB3D6462D385923557487844DF66A` _encounterid) (`EncounterActors_8_CE5BFEFA4BF41E1F55D63087C979553D` _encounteractors)) (break `/Game/Scripts/Data/S_Encounter` (`self.TargetEncounter`)))
  (if (`KismetArrayLibrary.Array_Contains` (`self.CompletedEncounters`) EncounterID)
    (`KismetSystemLibrary.PrintString` "Encounter Already Completed")
    (else
      (for _array_element (`self.LevelEncounters`)
        (if (== (`local.EncounterID`) (`.EncounterID_4_43AAB3D6462D385923557487844DF66A` (break `/Game/Scripts/Data/S_Encounter` _array_element)))
          (set `self.TargetEncounter` _array_element)
          (break)))
      (if (!= _encounterid -1)
        (for _array_element_2 _encounteractors
          (bind _returnvalue (`self.GetComponentByClass` _array_element_2 "/Game/Scripts/Components/BPC_TargetComponent.BPC_TargetComponent_C"))
          (add `/Game/Scripts/Components/BPC_TargetComponent.ETargetDestroyed` _returnvalue (`|CreateDelegate` :!event `OnTargetDestroyed`))
          (`/Engine/EditorBlueprintResources/StandardMacros.IncrementInt` (`self.CurrentTargetCount`)
            (:`  `
              (`/Game/Scripts/Components/BPC_TargetComponent.ActivateTarget` _returnvalue))))
        (`KismetSystemLibrary.PrintString` (`KismetStringLibrary.Concat_StrStr` (`KismetStringLibrary.Concat_StrStr` "Encounter " (`KismetStringLibrary.Conv_IntToString` (`.EncounterID_4_43AAB3D6462D385923557487844DF66A` (break `/Game/Scripts/Data/S_Encounter` (`self.TargetEncounter`)))) " Started: ") (`KismetStringLibrary.Conv_IntToString` (`self.CurrentTargetCount`)) " targets"))
        (`self.EEncounterStarted` (`self.CurrentTargetCount`))
        (for _array_element_3 (`.StartInteractors_19_F90DA5D342B27D851408BCBD22510FD4` (break `/Game/Scripts/Data/S_Encounter` (`self.TargetEncounter`)))
          (message `/Game/Scripts/Interfaces/BPI_Interact.Interact` _array_element_3 null))))))

(fn `DisableTarget`
  (params (TargetActor :type "Actor Object Reference"))
  (`self.SetActorTickEnabled` TargetActor false)
  (`self.SetActorHiddenInGame` TargetActor true))

(fn `EnableTarget`
  (params (TargetActor :type "Actor Object Reference"))
  (`self.SetActorTickEnabled` TargetActor true)
  (`self.SetActorHiddenInGame` TargetActor false))

(fn `UserConstructionScript`)