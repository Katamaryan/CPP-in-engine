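; Player tank Character that drives by rotating its tracks and moving along their forward vector, while the turret core yaws toward the cursor hit each tick.
; Firing spawns BP_TankShot through nested FlipFlops that alternate two guns and their four muzzle points, with timeline recoil and a short DoOnce cooldown.
; The health component's death event disables movement, hides the tank and starts a timer to respawn it at its BeginPlay location.
; BeginPlay also creates the main HUD widget.
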(event `self.ReceiveBeginPlay`
  (bind _bpc_cpphealthcomponent (`self.BPC_CPPHealthComponent`))
  ;[0.15 0.8348 0.15 0.5] BeginPlay
  (`self.SetRespawnPoint`)
  (`/Game/StudentWork/BPC_CPPHealthComponent.ResetHealth` _bpc_cpphealthcomponent)
  (add `/Game/StudentWork/BPC_CPPHealthComponent.EDeath` _bpc_cpphealthcomponent (`|CreateDelegate` :!event `TankDestroyed`))
  (`self.CreateHUD`))

(event `FireProjectile`
  (params (FirePoint :type "ArrowComponent Object Reference") (Gun01 :type Boolean))
  (bind (_returnvalue_location _returnvalue_rotation) (`KismetMathLibrary.BreakTransform` (`SceneComponent.K2_GetComponentToWorld` FirePoint)))
  ; FireProjectile
  (`|SpawnActorFromClass` "/Game/Scripts/Gameplay/Weapons/BP_TankShot.BP_TankShot_C" (`KismetMathLibrary.MakeTransform` _returnvalue_location _returnvalue_rotation) "AlwaysSpawn" "OverrideRootScale" null null)
  (`GameplayStatics.SpawnEmitterAtLocation` "/Game/Assets/Effects/PS_ShotBase.PS_ShotBase" _returnvalue_location _returnvalue_rotation)
  (`|ExecutionSequence`
    (:`then_0`
      (if Gun01
        (bind (_direction _newtrack_0) (`Timeline|Gun1Shudder` :!via `PlayFromStart`)
          (:`Update`
            (`SceneComponent.K2_SetRelativeLocation` (`self.TGun01`) (`KismetMathLibrary.MakeVector` _newtrack_0 15.0) false false)))
        (else
          (bind (_direction_2 _newtrack_0_2) (`Timeline|Gun2Shudder` :!via `PlayFromStart`)
            (:`Update`
              (`SceneComponent.K2_SetRelativeLocation` (`self.TGun02`) (`KismetMathLibrary.MakeVector` _newtrack_0_2 -15.0) false false))))))
    (:`then_1`
      (`KismetSystemLibrary.Delay` 0.2)
      (`self.ResetFire`))))

(event `self.IPrimaryAction`
  (params (inputClick :type Boolean))
  ;[0.7652 0.15 0.15 0.5] IA_Fire
  (if inputClick
    (if (not (`HealthComponent.bIsDead` (`self.BPC_CPPHealthComponent`)))
      (`/Engine/EditorBlueprintResources/StandardMacros.DoOnce` false :!label _label
        (:`Completed`
          (`/Engine/EditorBlueprintResources/StandardMacros.FlipFlop`
            (:`A`
              (`/Engine/EditorBlueprintResources/StandardMacros.FlipFlop`
                (:`A`
                  (`self.FireProjectile` (`self.W1`) true))
                (:`B`
                  (`self.FireProjectile` (`self.W2`) true))))
            (:`B`
              (`/Engine/EditorBlueprintResources/StandardMacros.FlipFlop`
                (:`A`
                  (`self.FireProjectile` (`self.W3`)))
                (:`B`
                  (`self.FireProjectile` (`self.W4`)))))))))))

(event `ResetFire`
  ;[0.7652 0.15 0.15 0.5] IA_Fire
  (goto _label :!via `Reset`))

(event `self.ReceiveTick`
  (params (DeltaSeconds :type "Float (single-precision)"))
  (bind (_returnvalue_x _returnvalue_y _returnvalue_z) (`KismetMathLibrary.BreakVector` (`SceneComponent.K2_GetComponentLocation` (`self.TCore01`))))
  ;[0.7652 0.15 0.15 0.5] IA_Fire
  (`SceneComponent.K2_SetWorldRotation` (`self.TCore01`) (`KismetMathLibrary.FindLookAtRotation` (`SceneComponent.K2_GetComponentLocation` (`self.TCore01`)) (`KismetMathLibrary.MakeVector` (.x (`.Location` (`GameplayStatics.BreakHitResult` (`PlayerController.GetHitResultUnderCursorByChannel` (`GameplayStatics.GetPlayerController` 0) "TraceTypeQuery1" true)))) (.y (`.Location` (`GameplayStatics.BreakHitResult` (`PlayerController.GetHitResultUnderCursorByChannel` (`GameplayStatics.GetPlayerController` 0) "TraceTypeQuery1" true)))) _returnvalue_z)) false false))

(event `TankDestroyed`
  (params (Instigator :type "Controller Object Reference") (Causer :type "Actor Object Reference"))
  ; TankDestroyed
  (if (not (`KismetSystemLibrary.K2_IsValidTimerHandle` (`self.RespawnTimerHandle`)))
    (`CharacterMovementComponent.DisableMovement` (`self.CharacterMovement`))
    (`SceneComponent.SetVisibility` (`self.CapsuleComponent`) false true)
    (`GameplayStatics.SpawnEmitterAtLocation` "/Game/Assets/Effects/PS_Dead.PS_Dead" (`self.K2_GetActorLocation`))
    (bind _returnvalue (`KismetSystemLibrary.K2_SetTimerDelegate` (`|CreateDelegate` :!event `Respawn`) (`self.RespawnTime`)))
    (set `self.RespawnTimerHandle` _returnvalue)))

(event `self.IMove`
  (params (inputValue :type "Float (single-precision)"))
  ;[0.7652 0.15 0.15 0.5] IA_Forward && IA_Turn
  (`self.AddMovementInput` (* inputValue (`KismetMathLibrary.Conv_RotatorToVector` (`SceneComponent.K2_GetComponentRotation` (`self.RotTracks`)))) 0.5))

(event `Respawn`
  ; TankDestroyed
  (`self.K2_SetActorLocation` (`self.RestartPoint`))
  (`/Game/StudentWork/BPC_CPPHealthComponent.ResetHealth` (`self.BPC_CPPHealthComponent`))
  (`CharacterMovementComponent.SetMovementMode` (`self.CharacterMovement`) "MOVE_Walking" 0)
  (`SceneComponent.SetVisibility` (`self.CapsuleComponent`) true true))

(event `self.ITurn`
  (params (inputValue :type "Float (single-precision)"))
  ;[0.7652 0.15 0.15 0.5] IA_Forward && IA_Turn
  (`SceneComponent.K2_AddRelativeRotation` (`self.RotTracks`) (`KismetMathLibrary.MakeRotator` 0.0 0.0 inputValue) false false))

(fn `CreateHUD`
  (bind _returnvalue (`|CreateWidget` "/Game/Scripts/UI/WBP_MainUI.WBP_MainUI_C" null self))
  (`UserWidget.AddToViewport` _returnvalue 0))

(fn `SetRespawnPoint`
  (bind (_returnvalue_x _returnvalue_y _returnvalue_z) (`KismetMathLibrary.BreakVector` (`self.K2_GetActorLocation`)))
  (set `self.RestartPoint` (`KismetMathLibrary.MakeVector` _returnvalue_x _returnvalue_y (+ _returnvalue_z 50.0))))

(fn `UserConstructionScript`)