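; Blueprint health component, apparently built on a C++ parent, that tracks damage and death for its owning actor.
; It binds to the owner's OnTakeAnyDamage on BeginPlay.
; ApplyDamage ignores dead or invulnerable owners, otherwise clamps health, broadcasts the change and checks for death.
; ResetHealth and CheckDeath extend their parent versions by firing health-modified and death dispatchers.
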(event `self.ReceiveBeginPlay`
  (add `Actor.OnTakeAnyDamage` (`self.GetOwner`) (`|CreateDelegate` :!event `ApplyDamage`)))

(event `self.ResetHealth`
  (`parent.ResetHealth`)
  (`self.EHealthModified` false (`self.CurrentHealth`) 0.0 1.0))

(event `self.CheckDeath`
  (params (Instigator :type "Controller Object Reference") (Causer :type "Actor Object Reference"))
  (`parent.CheckDeath` Instigator Causer)
  (if (`self.bIsDead`)
    (`self.EDeath` Instigator Causer)))

(fn `ApplyDamage`
  (params (DamagedActor :type "Actor Object Reference") (Damage :type "Float (single-precision)") (DamageType :type "DamageType Object Reference") (InstigatedBy :type "Controller Object Reference") (DamageCauser :type "Actor Object Reference"))
  (bind _damage (`local.Damage`))
  (if (not (or (`self.bIsDead`) (`self.bIsInvulnerable`)))
    (bind _output_get (set `self.CurrentHealth` (`KismetMathLibrary.FClamp` (- (`self.CurrentHealth`) Damage) 0.0 (`self.MaxHealth`))))
    (`self.EHealthModified` (> _damage 0.0) _output_get _damage (/ (`self.CurrentHealth`) (`self.MaxHealth`)))
    (`self.CheckDeath` (`local.InstigatedBy`) (`local.DamageCauser`))))